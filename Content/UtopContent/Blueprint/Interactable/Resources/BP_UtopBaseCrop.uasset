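; BP_UtopBaseCrop is a base farm crop interactable that grows through a list of stage meshes.
; Interacting removes its state tag, advances ProgressionState (wrapping after the last mesh) and starts cooldown timers by function name.
; SetReady then swaps the mesh, tags it Ready or Harvest, refreshes interactable messages and plays a Z-scale pop timeline.
; Setting the progression state also calls SetReady to update the crop immediately.
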(event `PopFarmPlot`
  (bind (_direction _newtrack_0) (`Timeline|PopPlot` :!via `PlayFromStart`)
    (:`Update`
      (`SceneComponent.SetRelativeScale3D` (`self.Mesh`) (`KismetMathLibrary.MakeVector` 1.0 1.0 _newtrack_0)))))

(event `self.ReceiveSetProgressionsState`
  (params (Progression :type "Float (single-precision)"))
  (`parent.ReceiveSetProgressionsState` Progression)
  (`self.Set Ready`))

(fn `Farming Progress`
  (returns (Delay :type "Float (double-precision)") (Stage :type Integer))
  (bind _cooldowntime (`self.CooldownTime`))
  (bind _returnvalue (`KismetMathLibrary.FTrunc` (`self.ProgressionState`)))
  (`|ExecutionSequence`
    (:`then_0`
      (`KismetArrayLibrary.Array_Remove` (`self.Tags`) 1))
    (:`then_1`
      (`KismetSystemLibrary.K2_SetTimer` null "Switch Stage" _cooldowntime))
    (:`then_2`
      (bind _output_get (set `self.ProgressionState` (`KismetMathLibrary.Conv_IntToDouble` (`KismetMathLibrary.SelectInt` 0 (+ _returnvalue 1) (>= _returnvalue (`KismetArrayLibrary.Array_LastIndex` (`self.MeshList`)))))))
      (return _cooldowntime (`KismetMathLibrary.FTrunc` _output_get)))))

(fn `ReceiveInteract`
  (returns (InCollectionTime :type "Float (single-precision)"))
  (`parent.ReceiveInteract`)
  (bind _delay (`self.Farming Progress`))
  (return _delay))

(fn `Set Ready`
  (`KismetArrayLibrary.Array_Set` (`self.Tags`) 1 (select `bool` (== (`KismetArrayLibrary.Array_LastIndex` (`self.MeshList`)) (`KismetMathLibrary.FFloor` (`self.ProgressionState`))) :`false` "Ready" :`true` "Harvest" :!type "Name") true)
  (`StaticMeshComponent.SetStaticMesh` (`self.Mesh`) (`|GetArrayItem` (`self.MeshList`) (`KismetMathLibrary.FTrunc` (`self.ProgressionState`))))
  (message `GameInstanceInterface.UpdateAllInteractables` (`GameplayStatics.GetGameInstance`))
  (`self.PopFarmPlot`))

(fn `Switch Stage`
  (if (== 0 (`KismetMathLibrary.FFloor` (`self.ProgressionState`)))
    (`self.Set Ready`)
    (else
      (`KismetSystemLibrary.K2_SetTimer` null "Set Ready" (`self.CooldownTime`)))))

(fn `UserConstructionScript`
  (`parent.UserConstructionScript`)
  (set `self.Tags` (`|MakeArray` "Farming" "Ready" :!type "Name")))